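; Parent zombie Blueprint that runs at a referenced wall and removes itself on arrival or death.
; On BeginPlay it turns its mesh toward BPWall, loops a run animation and uses AIMoveTo to approach.
; On arrival it screams, plays sounds, fires a Niagara burst, hides and destroys itself, applying no damage here.
; AnyDamage lowers Hp; at zero it plays death sound and animation, then destroys the actor after a delay.
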(event `self.ReceiveBeginPlay`
  ;[0.06582 0.15 0.03875 0.5] Move_To
  (`SceneComponent.K2_SetRelativeRotation` (`self.Mesh`) (`KismetMathLibrary.FindLookAtRotation` (`self.K2_GetActorLocation`) (`self.K2_GetActorLocation` (`self.BP_wall`))) false false)
  (`SkeletalMeshComponent.PlayAnimation` (`self.Mesh`) "/Game/Dev/Blueprint/Zombie/Zombie_Run_Anim.Zombie_Run_Anim" true)
  (`|AIMoveTo` self (`self.K2_GetActorLocation` (`self.BP_wall`)) null 130.0
    (:`OnSuccess`
      (`SkeletalMeshComponent.PlayAnimation` (`self.Mesh`) "/Game/Dev/Blueprint/Zombie/Zombie_Scream.Zombie_Scream" false)
      (`GameplayStatics.PlaySoundAtLocation` "/Game/Dev/Blueprint/Zombie/zombie-death-2-95167-_1___1_.zombie-death-2-95167-_1___1_" (`self.K2_GetActorLocation`) (struct) 1.0 1.0 0.0 null null null null)
      (`KismetSystemLibrary.Delay` 1.0)
      (`GameplayStatics.PlaySoundAtLocation` "/Game/Dev/Blueprint/Zombie/hit-flesh-02-266309.hit-flesh-02-266309" (`self.K2_GetActorLocation`) (struct) 1.0 1.0 0.0 null null null null)
      (`ActorComponent.Activate` (`self.NS_Simple_Burst_Level_3`) false)
      (`SceneComponent.SetVisibility` (`self.Mesh`) false false)
      (`KismetSystemLibrary.Delay` 0.7)
      (`self.K2_DestroyActor`))))

(event `self.ReceiveAnyDamage`
  (params (Damage :type "Float (single-precision)") (DamageType :type "DamageType Object Reference") (InstigatedBy :type "Controller Object Reference") (DamageCauser :type "Actor Object Reference"))
  ;[0.15 0 0 0.5] IsDamaged?
  (bind _output_get (set `self.Hp` (`KismetMathLibrary.FClamp` (- (`self.Hp`) Damage) 0.0 (`self.Hp`))))
  (if (<= _output_get 0.0)
    (`GameplayStatics.PlaySoundAtLocation` "/Game/Dev/Blueprint/Zombie/zombie-death-2-95167-_1___1_.zombie-death-2-95167-_1___1_" (`self.K2_GetActorLocation`) (struct) 1.0 1.0 0.0 null null null null)
    (`SkeletalMeshComponent.PlayAnimation` (`self.Mesh`) "/Game/Dev/Blueprint/Zombie/Zombie_Death.Zombie_Death" false)
    (`KismetSystemLibrary.Delay` 1.5)
    (`self.K2_DestroyActor`)))

(fn `UserConstructionScript`)