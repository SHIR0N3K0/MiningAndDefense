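; BP_wall is a damageable wall in the Zombie folder whose destruction ends the game.
; On BeginPlay it stores its starting HP as MaxHP and pre-creates a WBP_GameEnd widget.
; AnyDamage subtracts damage from HP with a floor of zero.
; At zero HP it switches to UI-only input with a visible cursor, freezes play through global time dilation and shows the game-end widget.
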(event `self.ReceiveBeginPlay`
  (set `self.Max HP` (`self.HP`))
  (bind _returnvalue (`|CreateWidget` "/Game/Dev/Widget/WBP_GameEnd.WBP_GameEnd_C"))
  (set `self.WBP REF` _returnvalue))

(event `self.ReceiveAnyDamage`
  (params (Damage :type "Float (single-precision)") (DamageType :type "DamageType Object Reference") (InstigatedBy :type "Controller Object Reference") (DamageCauser :type "Actor Object Reference"))
  (bind _returnvalue (`GameplayStatics.GetPlayerController` 0))
  ;[0.15 0.08833 0.004129 0.5] Any_Damaged
  (set `self.Hp` (`KismetMathLibrary.FClamp` (- (`self.Hp`) Damage) 0.0 (`self.Hp`)))
  (if (<= (`self.Hp`) 0.0)
    (`WidgetBlueprintLibrary.SetInputMode_UIOnlyEx` _returnvalue (`self.WBP REF`))
    (set `PlayerController.bShowMouseCursor` true _returnvalue)
    (`GameplayStatics.SetGlobalTimeDilation` 0.0)
    (`UserWidget.AddToViewport` (`self.WBP REF`) 0)))

(fn `UserConstructionScript`)