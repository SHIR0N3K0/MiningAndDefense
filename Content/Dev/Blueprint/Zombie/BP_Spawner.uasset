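; BP_Spawner is a zombie wave spawner that sends growing waves against a target wall, one wave per night number.
; A looping timer started on BeginPlay waits a random few seconds, then spawns a count looked up from the night number.
; Each spawn picks a random zombie class and location point, receives the wall target, wave number and player's FPS flag, then starts moving.
; The night number increments after each wave.
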(event `self.ReceiveBeginPlay`
  (`KismetSystemLibrary.K2_SetTimerDelegate` (delegate `Tick`) (`self.Time`) true false (`self.Initial Start Delay`))
  (bind _asbp_third_person_character (cast `/Game/Dev/Blueprint/Player/BP_ThirdPersonCharacter` (`GameplayStatics.GetPlayerCharacter` 0)))
  (set `self.Player REF` _asbp_third_person_character))

(event `Tick`
  (`KismetSystemLibrary.Delay` (`KismetMathLibrary.RandomFloatInRange` 3.0 10.0))
  (`self.spawn`))

(event `spawn`
  (bind _zombie_list (`self.Zombie_list`))
  (bind _spawned_actor (`self.Spawned Actor`))
  (set `self.Nb_ennemie` (select `int` (`self.NightNumber`) :`0` 4 :`1` 8 :`2` 12 :`3` 16 :`4` 20 :`5` 28 :`6` 36 :`7` 44 :`8` 52 :`9` 60 :`10` 70 :`11` 80 :`12` 100 :`13` 120 :`14` 140 :`15` 160 :`16` 180 :`17` 200 :`18` 230 :`19` 260 :`20` 290 :`21` 320))
  (for _ (range (`self.Nb_ennemie`))
    (bind _returnvalue (`|SpawnActorFromClass` (`|GetArrayItem` _zombie_list (`KismetMathLibrary.RandomInteger` (`KismetArrayLibrary.Array_Length` _zombie_list))) (`KismetMathLibrary.MakeTransform` (`KismetArrayLibrary.Array_Random` (`self.Location_Point`))) "AdjustIfPossibleButAlwaysSpawn" "MultiplyWithRoot" null null))
    (bind _asbp_zombie_parent (cast `/Game/Dev/Blueprint/Zombie/BP_ZombieParent` _returnvalue))
    (set `self.Spawned Actor` _asbp_zombie_parent)
    (set `/Game/Dev/Blueprint/Zombie/BP_ZombieParent.TargetLocation` (`SceneComponent.K2_GetComponentLocation` (`/Game/Dev/Blueprint/Zombie/BP_wall.TargetPoint` (`self.Target Wall`))) _asbp_zombie_parent)
    (set `/Game/Dev/Blueprint/Zombie/BP_ZombieParent.IsPlayerInFps?` (`/Game/Dev/Blueprint/Player/BP_ThirdPersonCharacter.FPS?` (`self.Player REF`)) _spawned_actor)
    (set `/Game/Dev/Blueprint/Zombie/BP_ZombieParent.TargetActor` (`self.Target Wall`) _spawned_actor)
    (set `/Game/Dev/Blueprint/Zombie/BP_ZombieParent.ActualWave` (`self.NightNumber`) _spawned_actor)
    (`/Game/Dev/Blueprint/Zombie/BP_ZombieParent.StartMoving` _spawned_actor))
  (`/Engine/EditorBlueprintResources/StandardMacros.IncrementInt` (`self.NightNumber`)))

(fn `UserConstructionScript`)