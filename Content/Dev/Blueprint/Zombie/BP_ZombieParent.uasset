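; Parent zombie Blueprint that walks to a target location and attacks the target actor by sacrificing itself.
; StartMoving runs AI MoveTo, then screams, deals its remaining HP as damage and destroys itself, adding impact sound and burst effect only in FPS view.
; HP scales with the current wave; damage flashes a hurt material and triggers a one-time death at zero.
; A looping timer mutes audio outside FPS view.
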(event `StartMoving`
  (bind _audio (`self.Audio`))
  (bind _targetactor (`self.TargetActor`))
  (`|AIMoveTo` self (`self.TargetLocation`) null 150.0
    (:`OnSuccess`
      (`SkeletalMeshComponent.PlayAnimation` (`self.Mesh`) "/Game/Dev/Blueprint/Zombie/Zombie_Scream.Zombie_Scream" false)
      (if (`self.IsPlayerInFps?`)
        (`AudioComponent.SetSound` _audio "/Game/Dev/Blueprint/Zombie/zombie-death-2-95167-_1___1_.zombie-death-2-95167-_1___1_")
        (`KismetSystemLibrary.Delay` 0.95)
        (`AudioComponent.SetSound` _audio "/Game/Dev/Blueprint/Zombie/hit-flesh-02-266309.hit-flesh-02-266309")
        (`ActorComponent.Activate` (`self.NS_Simple_Burst_Level_3`) false))
      (`/Engine/EditorBlueprintResources/StandardMacros.IsValid` _targetactor
        (:`Is Valid`
          (`GameplayStatics.ApplyDamage` _targetactor (`self.HP`))
          (`SceneComponent.SetVisibility` (`self.Mesh`) false false)
          (`AudioComponent.SetVolumeMultiplier` (`self.Audio`) 0.0)
          (`KismetSystemLibrary.Delay` 0.4)
          (`self.K2_DestroyActor`))))))

(event `self.ReceiveBeginPlay`
  (`KismetSystemLibrary.K2_SetTimerDelegate` (delegate `Check`) 0.5 true)
  (set `CharacterMovementComponent.MaxWalkSpeed` (`self.Speed`) (`self.CharacterMovement`))
  (`KismetSystemLibrary.Delay` 0.1)
  (set `self.HP` (* (`self.HP`) (+ (/ (`self.ActualWave`) 10) 1))))

(event `Check`
  (`AudioComponent.SetVolumeMultiplier` (`self.Audio`) (select `bool` (`self.IsPlayerInFps?`) :`true` 0.8 :!type "Float (single-precision)")))

(event `self.ReceiveAnyDamage`
  (params (Damage :type "Float (single-precision)") (DamageType :type "DamageType Object Reference") (InstigatedBy :type "Controller Object Reference") (DamageCauser :type "Actor Object Reference"))
  (set `self.HP` (- (`self.HP`) Damage))
  (`|ExecutionSequence`
    (:`then_0`
      (`PrimitiveComponent.SetMaterial` (`self.Mesh`) 0 "/Game/Dev/Blueprint/Zombie/M_Hurt.M_Hurt")
      (`KismetSystemLibrary.RetriggerableDelay` 0.2)
      (`PrimitiveComponent.SetMaterial` (`self.Mesh`) 0 "/Game/Dev/Blueprint/Zombie/Ch10_body.Ch10_body"))
    (:`then_1`
      (if (<= (`self.HP`) 0.0)
        (`/Engine/EditorBlueprintResources/StandardMacros.DoOnce` false
          (:`Completed`
            (`CharacterMovementComponent.DisableMovement` (`self.CharacterMovement`))
            (`AudioComponent.SetSound` (`self.Audio`) "/Game/Dev/Blueprint/Zombie/zombie-death-2-95167-_1___1_.zombie-death-2-95167-_1___1_")
            (`SkeletalMeshComponent.PlayAnimation` (`self.Mesh`) "/Game/Dev/Blueprint/Zombie/Zombie_Death.Zombie_Death" false)
            (`KismetSystemLibrary.Delay` 3.0)
            (`self.K2_DestroyActor`)))))))

(fn `UserConstructionScript`)