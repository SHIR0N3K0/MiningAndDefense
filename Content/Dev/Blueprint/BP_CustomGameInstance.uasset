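; Custom game instance that centralizes menu actions and player settings for audio and video.
; Play removes the calling widget, switches to game-only input and opens the test level, while Exit quits the game.
; Volume events apply sound class overrides for master, music and SFX on the master audio mix.
; Resolution, screen mode and graphics quality events update Game User Settings and apply them immediately.
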(event `/Game/Dev/Widget/BPI_MenuLogic.Play Game`
  (params (WidgetToRemove :type "Widget Object Reference"))
  (`Widget.RemoveFromParent` WidgetToRemove)
  (`WidgetBlueprintLibrary.SetInputMode_GameOnly` (`GameplayStatics.GetPlayerController` 0))
  (`GameplayStatics.OpenLevelBySoftObjectPtr` "/Game/GD/Lvl_Test.Lvl_Test"))

(event `/Game/Dev/Widget/BPI_MenuLogic.ExitGame`
  (`KismetSystemLibrary.QuitGame` null "Quit"))

(event `/Game/Dev/Widget/BPI_MenuLogic.UpdateMasterVolume`
  (params (NewVolume :type "Float (double-precision)"))
  (`GameplayStatics.SetSoundMixClassOverride` "/Game/Audio/Game_AudioMasterMix.Game_AudioMasterMix" "/Game/Audio/Game_AudioMaster.Game_AudioMaster" NewVolume))

(event `/Game/Dev/Widget/BPI_MenuLogic.UpdateMusicVolume`
  (params (`New Volume` :type "Float (double-precision)"))
  (`GameplayStatics.SetSoundMixClassOverride` "/Game/Audio/Game_AudioMasterMix.Game_AudioMasterMix" "/Game/Audio/Game_Music.Game_Music" `New Volume`))

(event `/Game/Dev/Widget/BPI_MenuLogic.UpdateSfxVolume`
  (params (`New Volume` :type "Float (double-precision)"))
  (`GameplayStatics.SetSoundMixClassOverride` "/Game/Audio/Game_AudioMasterMix.Game_AudioMasterMix" "/Game/Audio/Game_SFX.Game_SFX" `New Volume`))

(event `/Game/Dev/Widget/BPI_MenuLogic.Update ScreenResolution`
  (params (NewResolution :type "IntPoint Structure"))
  (bind _returnvalue (`GameUserSettings.GetGameUserSettings`))
  (`GameUserSettings.SetScreenResolution` _returnvalue NewResolution)
  (`GameUserSettings.ApplySettings` _returnvalue false))

(event `/Game/Dev/Widget/BPI_MenuLogic.UpdateScreenMode`
  (params (ScreenMode :type "EWindowMode Enum" :default "Fullscreen"))
  (bind _returnvalue (`GameUserSettings.GetGameUserSettings`))
  (`GameUserSettings.SetFullscreenMode` _returnvalue ScreenMode)
  (`GameUserSettings.ApplySettings` _returnvalue false))

(event `/Game/Dev/Widget/BPI_MenuLogic.UpdateGraphicsLevel`
  (params (NewQuality :type Integer))
  (bind _returnvalue (`GameUserSettings.GetGameUserSettings`))
  (`GameUserSettings.SetOverallScalabilityLevel` _returnvalue NewQuality)
  (`GameUserSettings.ApplySettings` _returnvalue false))