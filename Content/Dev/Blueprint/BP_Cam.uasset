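; BP_Cam is a camera rig actor that follows a third-person player horizontally.
; StartFolow stores the player reference, and each Tick moves the SpringArm to the player's X and Y while keeping its own world Z, so vertical movement is ignored.
; The TargetArmLength variable sets the spring arm length in both the construction script and BeginPlay.
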(event `self.ReceiveBeginPlay`
  (set `SpringArmComponent.TargetArmLength` (`self.Target Arm Length`) (`self.SpringArm`)))

(event `self.ReceiveTick`
  (params (DeltaSeconds :type "Float (single-precision)"))
  (bind (_returnvalue_x _returnvalue_y) (`KismetMathLibrary.BreakVector` (`self.K2_GetActorLocation` (`self.TPS Player REF`))))
  (bind (_returnvalue_x_2 _returnvalue_y_2 _returnvalue_z) (`KismetMathLibrary.BreakVector` (`SceneComponent.K2_GetComponentLocation` (`self.SpringArm`))))
  (`/Engine/EditorBlueprintResources/StandardMacros.IsValid` (`self.TPS Player REF`)
    (:`Is Valid`
      (`SceneComponent.K2_SetWorldLocation` (`self.SpringArm`) (`KismetMathLibrary.MakeVector` _returnvalue_x _returnvalue_y _returnvalue_z) false false))))

(event `StartFolow`
  (params (`TPS Player REF` :type "/Game/Dev/Blueprint/BP_ThirdPersonCharacter Object Reference"))
  (set `self.TPS Player REF` `TPS Player REF`))

(fn `UserConstructionScript`
  (set `SpringArmComponent.TargetArmLength` (`self.Target Arm Length`) (`self.SpringArm`)))