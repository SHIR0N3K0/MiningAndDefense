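; Player-mountable upgradeable turret: Interact toggles the player in or out, swapping view target and player mesh visibility.
; While manned, Tick turns it along the player's camera and line-traces an aim point.
; Fire runs a looping timer that staggers sphere-trace shots across up to four barrels, revealing extra barrel meshes as used.
; UpdateLevel derives barrel count, damage and fire rate from level; top-level shots deal area damage at impact.
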(event `self.ReceiveBeginPlay`
  (`SceneComponent.SetVisibility` (`self.SM_DownRight`) false false)
  (`SceneComponent.SetVisibility` (`self.SM_UpLeft`) false false)
  (`SceneComponent.SetVisibility` (`self.SM_UpRight`) false false))

(event `self.ReceiveTick`
  (params (DeltaSeconds :type "Float (single-precision)"))
  (bind _returnvalue (`self.K2_GetActorLocation`))
  (bind _player_ref (`self.Player REF`))
  (bind _camera (`self.Camera`))
  (bind _returnvalue_2 (`SceneComponent.K2_GetComponentLocation` _camera))
  (`/Engine/EditorBlueprintResources/StandardMacros.IsValid` _player_ref
    (:`Is Valid`
      (if (`/Game/Dev/Blueprint/Player/BP_ThirdPersonCharacter.Turret?` _player_ref)
        (`self.K2_SetActorRotation` (`KismetMathLibrary.FindLookAtRotation` _returnvalue (+ _returnvalue (* (`SceneComponent.GetForwardVector` (`/Game/Dev/Blueprint/Player/BP_ThirdPersonCharacter.FollowCamera` _player_ref)) 2000.0))))
        (bind _outhit (`KismetSystemLibrary.LineTraceSingle` _returnvalue_2 (+ _returnvalue_2 (* (`SceneComponent.GetForwardVector` _camera) 10000.0)) "TraceTypeQuery1"))
        (set `self.ForwardPoint` (`.ImpactPoint` (`GameplayStatics.BreakHitResult` _outhit)))))))

(event `/Game/Dev/Blueprint/BPI_Interact.Interact`
  (params (Messager :type "/Game/Dev/Blueprint/Player/BP_ThirdPersonCharacter Object Reference"))
  (bind _output_get (set `self.Player REF` Messager))
  (if (`/Game/Dev/Blueprint/Player/BP_ThirdPersonCharacter.Turret?` _output_get)
    (set `/Game/Dev/Blueprint/Player/BP_ThirdPersonCharacter.Turret?` false _output_get)
    (`SceneComponent.SetVisibility` (`Character.Mesh` _output_get) true false)
    (`PlayerController.SetViewTargetWithBlend` (`GameplayStatics.GetPlayerController` 0) _output_get 0.5 "VTBlend_Linear" 0.0 false)
    (`/Game/Dev/Blueprint/Player/BP_ThirdPersonCharacter.FPS_View` _output_get)
    (else
      (set `/Game/Dev/Blueprint/Player/BP_ThirdPersonCharacter.Turret?` true _output_get)
      (`SceneComponent.SetVisibility` (`Character.Mesh` _output_get) false false)
      (`PlayerController.SetViewTargetWithBlend` (`GameplayStatics.GetPlayerController` 0) self 0.5 "VTBlend_Linear" 0.0 false)
      (`/Game/Dev/Blueprint/Player/BP_ThirdPersonCharacter.TurretView` _output_get))))

(event `/Game/Dev/Blueprint/BPI_Interact.Fire`
  (params (WhoFire :type "/Game/Dev/Blueprint/Player/BP_ThirdPersonCharacter Object Reference"))
  ; Fire
  (if (`/Game/Dev/Blueprint/Player/BP_ThirdPersonCharacter.Turret?` WhoFire)
    (if (`/Game/Dev/Blueprint/Player/BP_ThirdPersonCharacter.Pressed?` WhoFire)
      (bind _returnvalue (`KismetSystemLibrary.K2_SetTimerDelegate` (delegate `Shoot`) (/ 1.0 (`self.FireRate`)) true))
      (set `self.TimerHandle` _returnvalue)
      (else
        (`KismetSystemLibrary.K2_ClearAndInvalidateTimerHandle` (`self.TimerHandle`))))))

(event `Shoot`
  (bind _nb_turret (`self.NB Turret`))
  (bind _nb_turret_2 (`self.NB Turret`))
  (bind _nb_turret_3 (`self.NB Turret`))
  ; Fire
  (`self.FireTrace` (`self.ArrowDownLeft`))
  (if (>= _nb_turret_3 2)
    (`SceneComponent.SetVisibility` (`self.SM_DownRight`) true false)
    (`KismetSystemLibrary.Delay` (/ (/ 1.0 (`self.FireRate`)) (select `int` _nb_turret_3 :`0` 0.0 :`1` 0.0 :`2` 2.0 :`3` 3.0 :`4` 4.0)))
    (`self.FireTrace` (`self.ArrowDownRight`))
    (if (>= _nb_turret 3)
      (`SceneComponent.SetVisibility` (`self.SM_UpLeft`) true false)
      (`KismetSystemLibrary.Delay` (/ (/ 1.0 (`self.FireRate`)) (select `int` _nb_turret :`0` 0.0 :`1` 0.0 :`2` 2.0 :`3` 3.0 :`4` 4.0)))
      (`self.FireTrace` (`self.ArrowUpRight`))
      (if (>= _nb_turret_2 4)
        (`SceneComponent.SetVisibility` (`self.SM_UpRight`) true false)
        (`KismetSystemLibrary.Delay` (/ (/ 1.0 (`self.FireRate`)) (select `int` _nb_turret_2 :`0` 0.0 :`1` 0.0 :`2` 2.0 :`3` 3.0 :`4` 4.0)))
        (`self.FireTrace` (`self.ArrowUpLeft`))))))

(event `UpdateLevel`
  ; Update Level
  (set `self.NB Turret` (select `int` (`self.LevelTurret`) :`0` 0 :`1` 1 :`2` 1 :`3` 2 :`4` 2 :`5` 3 :`6` 4))
  (set `self.TurretDamage` (select `int` (`self.LevelTurret`) :`0` 0.0 :`1` 10.0 :`2` 20.0 :`3` 30.0 :`4` 50.0 :`5` 70.0 :`6` 120.0 :!type "Float (single-precision)"))
  (set `self.FireRate` (select `int` (`self.LevelTurret`) :`0` 0.0 :`1` 0.8 :`2` 1.4 :`3` 1.8 :`4` 2.3 :`5` 2.6 :`6` 3.0)))

(fn `FireTrace`
  (params (Target :type "SceneComponent Object Reference"))
  (if (< (`self.LevelTurret`) 6)
    (bind _outhit (`KismetSystemLibrary.SphereTraceSingleForObjects` :`Start` (`SceneComponent.K2_GetComponentLocation` Target) :`End` (`self.ForwardPoint`) :`Radius` 10.0 :`ObjectTypes` (`|MakeArray` "ObjectTypeQuery3" :!type "EObjectTypeQuery Enum") :`DrawDebugType` "Persistent"))
    (`GameplayStatics.ApplyDamage` (`.HitActor` (`GameplayStatics.BreakHitResult` _outhit)) (`self.TurretDamage`))
    (else
      (bind _outhit_2 (`KismetSystemLibrary.SphereTraceSingle` :`Start` (`SceneComponent.K2_GetComponentLocation` Target) :`End` (`self.ForwardPoint`) :`Radius` 10.0 :`TraceChannel` "TraceTypeQuery1" :`DrawDebugType` "ForOneFrame"))
      (`KismetArrayLibrary.Array_Clear` (`self.DamagedActor`))
      (bind (_bblockinghit _binitialoverlap _time _distance _location _impactpoint) (`GameplayStatics.BreakHitResult` _outhit_2))
      (bind _outhits (`KismetSystemLibrary.SphereTraceMultiForObjects` :`Start` _impactpoint :`End` _impactpoint :`Radius` (`self.RadiusExplosive bullet`) :`ObjectTypes` (`|MakeArray` "ObjectTypeQuery3" :!type "EObjectTypeQuery Enum") :`DrawDebugType` "ForOneFrame"))
      (for _array_element _outhits
        (bind (_bblockinghit_2 _binitialoverlap_2 _time_2 _distance_2 _location_2 _impactpoint_2 _normal _impactnormal _physmat _hitactor) (`GameplayStatics.BreakHitResult` _array_element))
        (if (not (`KismetArrayLibrary.Array_Contains` (`self.DamagedActor`) _hitactor))
          (`KismetArrayLibrary.Array_Add` (`self.DamagedActor`) _hitactor)
          (`GameplayStatics.ApplyDamage` _hitactor (`self.TurretDamage`)))))))

(fn `UserConstructionScript`)