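; Mine doorway actor, set as entry or exit by a flag, that teleports the player on interact while inside its trigger box.
; Entry switches game type and blends to a following camera with the character mesh visible; exit switches back to the character's view and hides the mesh.
; Exit instances add an exit marker widget and run a looping timer that has the breakable manager respawn rocks after a cooldown, once the exit has been used.
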(event `self.ReceiveBeginPlay`
  (if (not (`self.Entry`))
    (`KismetSystemLibrary.K2_SetTimerDelegate` (delegate `Timer`) 1.0 true))
  (if (not (`self.Entry`))
    (bind _returnvalue (`|CreateWidget` "/Game/Dev/Blueprint/Widget/WBP_ExitMarker.WBP_ExitMarker_C"))
    (set `/Game/Dev/Blueprint/Widget/WBP_ExitMarker.Targeted Comp` self _returnvalue)
    (`UserWidget.AddToViewport` _returnvalue 0)))

(event `Timer`
  (`/Engine/EditorBlueprintResources/StandardMacros.IncrementFloat` (`self.TimePassing`)
    (:`  `
      (if (> (`self.TimePassing`) 180.0)
        (set `self.Can Respawn Breakable` true)
        (set `self.TimePassing` 0.0))
      (if (and (`self.Can Respawn Breakable`) (`self.Exited`))
        (`/Game/Dev/Blueprint/Breakable/BP_BreakableManager.EventRockSpawnLocation` (`self.BreackableManager REF`))
        (set `self.Can Respawn Breakable` false)))))

(event `self.Box.OnComponentBeginOverlap`
  (params (OverlappedComponent :type "PrimitiveComponent Object Reference") (OtherActor :type "Actor Object Reference") (OtherComp :type "PrimitiveComponent Object Reference") (OtherBodyIndex :type Integer) (bFromSweep :type Boolean) (SweepResult :type "HitResult Structure (by ref)"))
  (cast `/Game/Dev/Blueprint/Player/BP_ThirdPersonCharacter` OtherActor)
  (`SceneComponent.SetVisibility` (`self.Widget`) true false)
  (set `self.InBox?` true))

(event `self.Box.OnComponentEndOverlap`
  (params (OverlappedComponent :type "PrimitiveComponent Object Reference") (OtherActor :type "Actor Object Reference") (OtherComp :type "PrimitiveComponent Object Reference") (OtherBodyIndex :type Integer))
  (cast `/Game/Dev/Blueprint/Player/BP_ThirdPersonCharacter` OtherActor)
  (`SceneComponent.SetVisibility` (`self.Widget`) false false)
  (set `self.InBox?` false))

(event `/Game/Dev/Blueprint/BPI_Interact.Interact`
  (params (Messager :type "/Game/Dev/Blueprint/Player/BP_ThirdPersonCharacter Object Reference"))
  (bind (_returnvalue_roll _returnvalue_pitch _returnvalue_yaw) (`KismetMathLibrary.BreakRotator` (`self.K2_GetActorRotation` (`self.Cam REF`))))
  (bind _mesh (`Character.Mesh` (`self.As BP Third Person Character`)))
  (if (`self.InBox?`)
    (set `self.As BP Third Person Character` Messager)
    (`/Game/Dev/Blueprint/Widget/WBP_HUD.ViewChanged` (`/Game/Dev/Blueprint/Player/BP_ThirdPersonCharacter.HUD REF` (`self.As BP Third Person Character`)))
    (`KismetSystemLibrary.Delay` 0.15)
    (`self.K2_TeleportTo` :`self` (`self.As BP Third Person Character`) :`DestLocation` (`KismetMathLibrary.TransformLocation` (`self.GetTransform`) (`self.MineLocation`)))
    (if (`self.Entry`)
      (`Controller.SetControlRotation` (`GameplayStatics.GetPlayerController` 0) (`KismetMathLibrary.MakeRotator` 0.0 0.0 _returnvalue_yaw))
      (`/Game/Dev/Blueprint/Player/BP_ThirdPersonCharacter.ChangeGameType` (`self.As BP Third Person Character`) false)
      (`/Engine/EditorBlueprintResources/StandardMacros.IsValid` (`self.Cam REF`)
        (:`Is Valid`
          (`MeshComponent.SetScalarParameterValueOnMaterials` _mesh "DefaultOpacity" 1.0)
          (set `self.Exited` false)
          (`PlayerController.SetViewTargetWithBlend` (`GameplayStatics.GetPlayerController` 0) (`self.Cam REF`) 0.5 "VTBlend_Linear" 0.0 false)
          (`/Game/Dev/Blueprint/Camera/BP_Cam.StartFolow` (`self.Cam REF`) (`self.As BP Third Person Character`))))
      (else
        (`/Game/Dev/Blueprint/Player/BP_ThirdPersonCharacter.ChangeGameType` (`self.As BP Third Person Character`) true)
        (`PlayerController.SetViewTargetWithBlend` (`GameplayStatics.GetPlayerController` 0) (`self.As BP Third Person Character`) 0.5 "VTBlend_Linear" 0.0 false)
        (set `self.Exited` true)
        (`MeshComponent.SetScalarParameterValueOnMaterials` _mesh "DefaultOpacity" 0.0)))))

(fn `UserConstructionScript`)