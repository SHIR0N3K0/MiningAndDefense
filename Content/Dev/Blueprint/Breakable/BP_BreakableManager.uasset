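; Manager actor that populates a mine with randomly typed BP_Breakable rocks on BeginPlay.
; EventRockSpawnLocation first calls ResetMine to destroy previous spawns and refill the pool of free locations from RockSpawnLocation.
; Each rock's type comes from a cumulative weighted roll over BaseApparitionChance in DT_Breakable, mapping row order to the type enum.
; Rocks spawn at random unused actor-relative locations with random yaw, and each used location leaves the pool.
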(event `self.ReceiveBeginPlay`
  (`self.EventRockSpawnLocation`))

(fn `EventRockSpawnLocation`
  (locals (Acumulator :type Integer) (MaxActorThatCanBeSpawned :type Integer :default 0) (RadomResult :type Integer :default 0) (UsedLocation :type "Vector Structure") (IndexToRemove :type Integer))
  (bind _returnvalue (`KismetArrayLibrary.Array_Length` (`self.RockSpawnLocation`)))
  (`self.ResetMine`)
  (set `local.MaxActorThatCanBeSpawned` _returnvalue)
  (for _ (range (+ (`KismetMathLibrary.Clamp` (- (`self.NumbStoneToSpawn`) 1) 0 _returnvalue) 1))
    (set `local.RadomResult` (`KismetMathLibrary.RandomIntegerInRange` 0 100))
    (set `local.Acumulator` 0)
    (bind _outrownames (`DataTableFunctionLibrary.GetDataTableRowNames` "/Game/Dev/Blueprint/StatAndInfo/DT_Breakable.DT_Breakable"))
    (for (_array_element _array_index) _outrownames
      (bind _returnvalue_2 (`|GetDataTableRow` "/Game/Dev/Blueprint/StatAndInfo/DT_Breakable.DT_Breakable" _array_element)
        (:`then`
          (bind _output_get (set `local.Acumulator` (+ (`local.Acumulator`) (`.BaseApparitionChance_6_89D3E6944AF22148633FD1A6918D5978` (break `/Game/Dev/Blueprint/StatAndInfo/Struct_Breakable` _returnvalue_2)))))
          (if (<= (`local.RadomResult`) _output_get)
            (set `self.Type To Spawn` (select `int` _array_index :`0` "NewEnumerator0" :`1` "NewEnumerator1" :`2` "NewEnumerator2" :`3` "NewEnumerator3" :`4` "NewEnumerator4" :`5` "NewEnumerator5" :!type "/Game/Dev/Blueprint/StatAndInfo/E_BreakableType Enum"))
            (break)))))
    (set `local.IndexToRemove` (`KismetMathLibrary.RandomIntegerInRange` 0 (- (`KismetArrayLibrary.Array_Length` (`self.UnusedLocation`)) 1)))
    (bind _returnvalue_3 (`|SpawnActorFromClass` "/Game/Dev/Blueprint/Breakable/BP_Breakable.BP_Breakable_C" (`KismetMathLibrary.MakeTransform` (`KismetMathLibrary.TransformLocation` (`self.GetTransform`) (`|GetArrayItem` (`self.UnusedLocation`) (`local.IndexToRemove`))) (`KismetMathLibrary.MakeRotator` 0.0 0.0 (`KismetMathLibrary.RandomFloatInRange` 0.0 360.0))) "Undefined" "MultiplyWithRoot" self null))
    (set `/Game/Dev/Blueprint/Breakable/BP_Breakable.BreakableType` (`self.Type To Spawn`) _returnvalue_3)
    (`/Game/Dev/Blueprint/Breakable/BP_Breakable.SetBaseParam` _returnvalue_3)
    (`KismetArrayLibrary.Array_Add` (`self.AllActorSpawned`) _returnvalue_3)
    (`KismetArrayLibrary.Array_Remove` (`self.UnusedLocation`) (`local.IndexToRemove`))
    (`/Engine/EditorBlueprintResources/StandardMacros.DecrementInt` (`local.MaxActorThatCanBeSpawned`))))

(fn `ResetMine`
  (`KismetArrayLibrary.Array_Clear` (`self.UnusedLocation`))
  (for _array_element (`self.AllActorSpawned`)
    (`/Engine/EditorBlueprintResources/StandardMacros.IsValid` _array_element
      (:`Is Valid`
        (`self.K2_DestroyActor` _array_element))))
  (set `self.UnusedLocation` (`self.RockSpawnLocation`))
  (`KismetArrayLibrary.Array_Clear` (`self.AllActorSpawned`)))

(fn `UserConstructionScript`)