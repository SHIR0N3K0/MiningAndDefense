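; BP_Breakable is a mineable actor whose type picks its mesh, color, name label, strength requirement and extraction time from DT_Breakable.
; The construction script previews the look, and BeginPlay reapplies it, loads the stats and hides the label.
; Overlaped briefly shows the label via a retriggerable delay.
; Clicked fills a mining progress widget for strong enough clickers, destroys the actor at full duration, and resets progress when clicks stop.
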(event `self.ReceiveBeginPlay`
  (`self.SetBaseParam`)
  (bind _aswbp_mining_time (cast `/Game/Dev/Blueprint/Widget/WBP_MiningTime` (`WidgetComponent.GetWidget` (`self.WidgetMiningTime`))))
  (set `self.As WBP Mining Time REF` _aswbp_mining_time))

(event `/Game/Dev/Blueprint/BPI_Interact.Overlaped`
  (params (Overlaper :type "/Game/Dev/Blueprint/BP_ThirdPersonCharacter Object Reference"))
  (`SceneComponent.SetVisibility` (`self.WidgetName`) true false)
  (`KismetSystemLibrary.RetriggerableDelay` 0.2)
  (`SceneComponent.SetVisibility` (`self.WidgetName`) false false))

(event `/Game/Dev/Blueprint/BPI_Interact.Clicked`
  (params (Clicker :type "/Game/Dev/Blueprint/BP_ThirdPersonCharacter Object Reference") (`Clicked Time` :type "Float (double-precision)"))
  (bind _as_wbp_mining_time_ref (`self.As WBP Mining Time REF`))
  (`|ExecutionSequence`
    (:`then_0`
      (`KismetSystemLibrary.RetriggerableDelay` 0.1)
      (`/Game/Dev/Blueprint/Widget/WBP_MiningTime.ResetPercentage` _as_wbp_mining_time_ref))
    (:`then_1`
      (if (>= (`/Game/Dev/Blueprint/BP_ThirdPersonCharacter.MiningStrenght` Clicker) (`self.Strenght Required`))
        (`/Game/Dev/Blueprint/Widget/WBP_MiningTime.UpdatePercentage` _as_wbp_mining_time_ref (`KismetMathLibrary.FClamp` (/ `Clicked Time` (`self.Extraction Duration`))))
        (if (>= `Clicked Time` (`self.Extraction Duration`))
          (`/Engine/EditorBlueprintResources/StandardMacros.DoOnce` false
            (:`Completed`
              (`self.K2_DestroyActor`))))))))

(fn `SetBaseParam`
  (bind _staticmesh (`self.StaticMesh`))
  (bind _returnvalue (`|GetDataTableRow` "/Game/Dev/Blueprint/DT_Breakable.DT_Breakable" (`KismetStringLibrary.Conv_StringToName` (`|GetEnumeratorNameAsString` (`self.BreakableType`))))
    (:`then`
      (bind (_breakabletype _baseapparitionchance _strenghtrequired _extractionduration _color _mesh) (break `/Game/Dev/Blueprint/Struct_Breakable` _returnvalue))
      (set `self.Base Apparition Chance` _baseapparitionchance)
      (set `self.Strenght Required` _strenghtrequired)
      (set `self.Extraction Duration` _extractionduration)
      (`StaticMeshComponent.SetStaticMesh` _staticmesh _mesh)
      (`PrimitiveComponent.SetMaterial` _staticmesh 0 "/Game/Dev/Blueprint/M_Breakable.M_Breakable")
      (bind _returnvalue_2 (`KismetMathLibrary.Conv_ColorToLinearColor` _color))
      (`MeshComponent.SetColorParameterValueOnMaterials` _staticmesh "Color" _returnvalue_2)
      (bind _aswbp_text (cast `/Game/Dev/Blueprint/Widget/WBP_Text` (`WidgetComponent.GetWidget` (`self.WidgetName`))))
      (bind _textblock_0 (`/Game/Dev/Blueprint/Widget/WBP_Text.TextBlock_0` _aswbp_text))
      (set `TextBlock.Text` (`KismetTextLibrary.Conv_StringToText` (`|GetEnumeratorNameAsString` (`self.BreakableType`))) _textblock_0)
      (set `TextBlock.ColorAndOpacity` (make `SlateColor` _returnvalue_2) _textblock_0)
      (`SceneComponent.SetVisibility` (`self.WidgetName`) false false))))

(fn `UserConstructionScript`
  (bind _staticmesh (`self.StaticMesh`))
  (bind _returnvalue (`|GetDataTableRow` "/Game/Dev/Blueprint/DT_Breakable.DT_Breakable" (`KismetStringLibrary.Conv_StringToName` (`|GetEnumeratorNameAsString` (`self.BreakableType`))))
    (:`then`
      (bind (_breakabletype _baseapparitionchance _strenghtrequired _extractionduration _color _mesh) (break `/Game/Dev/Blueprint/Struct_Breakable` _returnvalue))
      (`StaticMeshComponent.SetStaticMesh` _staticmesh _mesh)
      (`PrimitiveComponent.SetMaterial` _staticmesh 0 "/Game/Dev/Blueprint/M_Breakable.M_Breakable")
      (bind _returnvalue_2 (`KismetMathLibrary.Conv_ColorToLinearColor` _color))
      (`MeshComponent.SetColorParameterValueOnMaterials` _staticmesh "Color" _returnvalue_2)
      (bind _aswbp_text (cast `/Game/Dev/Blueprint/Widget/WBP_Text` (`WidgetComponent.GetWidget` (`self.WidgetName`))))
      (bind _textblock_0 (`/Game/Dev/Blueprint/Widget/WBP_Text.TextBlock_0` _aswbp_text))
      (set `TextBlock.Text` (`KismetTextLibrary.Conv_StringToText` (`|GetEnumeratorNameAsString` (`self.BreakableType`))) _textblock_0)
      (set `TextBlock.ColorAndOpacity` (make `SlateColor` _returnvalue_2) _textblock_0))))