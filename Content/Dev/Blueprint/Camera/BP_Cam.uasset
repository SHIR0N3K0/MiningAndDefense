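; Camera actor that follows a TPS player in the horizontal plane at fixed height, with an editable lock boundary.
; Each tick it copies player XY when under three lock points exist.
; Otherwise a ray-crossing test checks the camera against the polygon and, only when outside, moves it to player XY clamped to the polygon's bounding box.
; Debug lines draw the boundary; closest-point-on-polygon helpers sit in unexecuted logic.
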(event `self.ReceiveBeginPlay`
  (set `SpringArmComponent.TargetArmLength` (`self.Target Arm Length`) (`self.SpringArm`)))

(event `self.ReceiveTick`
  (params (DeltaSeconds :type "Float (single-precision)"))
  (`/Engine/EditorBlueprintResources/StandardMacros.IsValid` (`self.TPS Player REF`)
    (:`Is Valid`
      (`self.ClampCameraWithinBoundary`)
      (`self.DrawDebugLine`))))

(event `StartFolow`
  (params (`TPS Player REF` :type "/Game/Dev/Blueprint/Player/BP_ThirdPersonCharacter Object Reference"))
  (set `self.TPS Player REF` `TPS Player REF`))

(fn `ClampCameraWithinBoundary`
  (locals (Intersections :type Integer) (CamLocation :type "Vector Structure") (FlatCamLocation :type "Vector2D Structure") (Polygon2D :type "Array of Vector2D Structure") (i :type Integer) (j :type Integer) (Pi :type "Vector2D Structure") (Pj :type "Vector2D Structure") (Slope :type "Float (double-precision)") (Cond1 :type Boolean) (`Min X` :type "Float (double-precision)" :default 0.0) (`Max X` :type "Float (double-precision)") (`Min Y` :type "Float (double-precision)" :default 0.0) (`Max Y` :type "Float (double-precision)") (Closest :type "Vector2D Structure") (NewLocation :type "Vector Structure"))
  (bind (_pi_x _pi_y) (`KismetMathLibrary.BreakVector2D` (`local.Pi`)))
  (bind (_flatcamlocation_x _flatcamlocation_y) (`KismetMathLibrary.BreakVector2D` (`local.FlatCamLocation`)))
  (bind (_pj_x _pj_y) (`KismetMathLibrary.BreakVector2D` (`local.Pj`)))
  (bind _pj_x_2 (`KismetMathLibrary.BreakVector2D` (`local.Pj`)))
  (bind _pi_x_2 (`KismetMathLibrary.BreakVector2D` (`local.Pi`)))
  (bind (_flatcamlocation_x_2 _flatcamlocation_y_2) (`KismetMathLibrary.BreakVector2D` (`local.FlatCamLocation`)))
  (bind (_pi_x_3 _pi_y_2) (`KismetMathLibrary.BreakVector2D` (`local.Pi`)))
  (bind (_pj_x_3 _pj_y_2) (`KismetMathLibrary.BreakVector2D` (`local.Pj`)))
  (bind (_camlocation_x _camlocation_y) (`KismetMathLibrary.BreakVector` (`local.CamLocation`)))
  (bind (_pi_x_4 _pi_y_3) (`KismetMathLibrary.BreakVector2D` (`local.Pi`)))
  (bind _pi_x_5 (`KismetMathLibrary.BreakVector2D` (`local.Pi`)))
  (bind _flatcamlocation_x_3 (`KismetMathLibrary.BreakVector2D` (`local.FlatCamLocation`)))
  (bind _camera (`self.Camera`))
  (bind (_camlocation_x_2 _camlocation_y_2 _camlocation_z) (`KismetMathLibrary.BreakVector` (`local.CamLocation`)))
  (bind _returnvalue (`KismetArrayLibrary.Array_Length` (`local.Polygon2D`)))
  (bind (_returnvalue_x _returnvalue_y) (`KismetMathLibrary.BreakVector` (`self.K2_GetActorLocation` (`self.TPS Player REF`))))
  (bind (_returnvalue_x_2 _returnvalue_y_2) (`KismetMathLibrary.BreakVector` (`self.K2_GetActorLocation` (`self.TPS Player REF`))))
  (bind (_returnvalue_x_3 _returnvalue_y_3 _returnvalue_z) (`KismetMathLibrary.BreakVector` (`SceneComponent.K2_GetComponentLocation` _camera)))
  (bind (_output_x _output_y) (`KismetMathLibrary.BreakVector2D` (`|GetArrayItem` (`local.Polygon2D`))))
  ; If less than 3 Lock Position Do Nothing
  (if (< (`KismetArrayLibrary.Array_Length` (`self.CameraLock`)) 3)
    (`SceneComponent.K2_SetWorldLocation` _camera (`KismetMathLibrary.MakeVector` _returnvalue_x _returnvalue_y _returnvalue_z) false false)
    (else
      ; Get cam world location and make it 2D
      (set `local.CamLocation` (`SceneComponent.K2_GetComponentLocation` (`self.Camera`)))
      (set `local.FlatCamLocation` (`KismetMathLibrary.MakeVector2D` _camlocation_x _camlocation_y))
      ; Get All lock position and make them 2D
      (for _array_element (`self.CameraLock`)
        (`KismetArrayLibrary.Array_Add` (`local.Polygon2D`) (`KismetMathLibrary.MakeVector2D` (.x (`KismetMathLibrary.TransformLocation` (`self.GetTransform`) _array_element)) (.y (`KismetMathLibrary.TransformLocation` (`self.GetTransform`) _array_element)))))
      ; Is Point in polygon
      (set `local.Intersections` 0)
      (set `local.j` (- _returnvalue 1))
      (for _ (range (`local.i`) (+ _returnvalue 1))
        (set `local.Pi` (`|GetArrayItem` (`local.Polygon2D`) (`local.i`)))
        (set `local.Pj` (`|GetArrayItem` (`local.Polygon2D`) (`local.j`)))
        (set `local.Cond1` (!= (> _pi_y _flatcamlocation_y_2) (> _pj_y _flatcamlocation_y_2)))
        (set `local.Slope` (+ (/ (* (- _pj_x_2 _pi_x_2) (- _flatcamlocation_y _pi_y_2)) (- _pj_y_2 _pi_y_3)) _pi_x_5))
        (if (and (`local.Cond1`) (< _flatcamlocation_x_3 (`local.Slope`)))
          (`/Engine/EditorBlueprintResources/StandardMacros.IncrementInt` (`local.Intersections`))))
      (if (not (== (mod (`local.Intersections`) 2) 1))
        ; Calculate Bounding
        (bind _output_get (set `local.Min X` _output_x))
        (set `local.Max X` _output_get)
        (bind _output_get_2 (set `local.Min Y` _output_y))
        (set `local.Max Y` _output_get_2)
        (for _array_element_2 (`local.Polygon2D`)
          (set `local.Min X` (`KismetMathLibrary.FMin` (`local.Min X`) (`KismetMathLibrary.BreakVector2D` _array_element_2)))
          (set `local.Max X` (`KismetMathLibrary.FMax` (`local.Max X`) (`KismetMathLibrary.BreakVector2D` _array_element_2)))
          (set `local.Min Y` (`KismetMathLibrary.FMin` (`local.Min Y`) (`.Y` (`KismetMathLibrary.BreakVector2D` _array_element_2))))
          (set `local.Max Y` (`KismetMathLibrary.FMax` (`local.Max Y`) (`.Y` (`KismetMathLibrary.BreakVector2D` _array_element_2)))))
        ; SetLocation
        (`SceneComponent.K2_SetWorldLocation` (`self.Camera`) (`KismetMathLibrary.MakeVector` (`KismetMathLibrary.FClamp` _returnvalue_x_2 (`local.Min X`) (`local.Max X`)) (`KismetMathLibrary.FClamp` _returnvalue_y_2 (`local.Min Y`) (`local.Max Y`)) _camlocation_z) false false)))))

(fn `ClosestPointOnPolygon2D`
  (params (Point :type "Vector2D Structure") (Polygon :type "Array of Vector2D Structure"))
  (returns (ClosestPoint :type "Vector2D Structure"))
  (locals (MinDistSq :type "Float (double-precision)") (`Closest Point` :type "Vector2D Structure") (A :type "Vector2D Structure") (B :type "Vector2D Structure") (Candidate :type "Vector2D Structure") (DistSq :type "Float (double-precision)"))
  (set `local.MinDistSq` 1e+87)
  (set `local.Closest Point` Point)
  (for _index (range (+ (`KismetArrayLibrary.Array_Length` Polygon) 1))
    (set `local.A` (`|GetArrayItem` Polygon _index))
    (set `local.B` (`|GetArrayItem` Polygon (mod (+ _index 1) (`KismetArrayLibrary.Array_Length` Polygon))))
    (bind _return (`self.ClosestPointOnSegment2D` Point (`local.A`) (`local.B`)))
    (set `local.Candidate` _return)
    (set `local.DistSq` (`KismetMathLibrary.DistanceSquared2D` Point (`local.Candidate`)))
    (if (< (`local.DistSq`) (`local.MinDistSq`))
      (set `local.MinDistSq` (`local.DistSq`))
      (set `local.Closest Point` (`local.Candidate`))))
  (return (`local.Closest Point`)))

(fn `ClosestPointOnSegment2D`
  (params (P :type "Vector2D Structure") (A :type "Vector2D Structure") (B :type "Vector2D Structure"))
  (returns (Return :type "Vector2D Structure"))
  (locals (AB :type "Vector2D Structure") (`AB_SqrLen ` :type "Float (double-precision)") (T :type "Float (double-precision)"))
  (set `local.AB` (- A B))
  (set `local.AB_SqrLen ` (`KismetMathLibrary.VSize2DSquared` (`local.AB`)))
  (if (<= (`local.AB_SqrLen `) 0.1)
    (return A)
    (else
      (set `local.T` (/ (`KismetMathLibrary.DotProduct2D` (- P A) (`local.AB`)) (`local.AB_SqrLen `)))
      (set `local.T` (`KismetMathLibrary.FClamp` (`local.T`)))
      (return (* (+ A (`local.T`)) (`local.AB`))))))

(fn `DrawDebugLine`
  (locals (NextIndex :type Integer) (`World PointA` :type "Vector Structure") (`World PointB` :type "Vector Structure"))
  (bind _returnvalue (`KismetArrayLibrary.Array_Length` (`self.CameraLock`)))
  (if (not (< (`KismetArrayLibrary.Array_Length` (`self.CameraLock`)) 3))
    (for _index (range (+ _returnvalue 1))
      (set `local.NextIndex` (mod (+ _index 1) _returnvalue))
      (set `local.World PointA` (`KismetMathLibrary.TransformLocation` (`SceneComponent.GetRelativeTransform` (`self.DefaultSceneRoot`)) (`|GetArrayItem` (`self.CameraLock`) _index)))
      (set `local.World PointB` (`KismetMathLibrary.TransformLocation` (`SceneComponent.GetRelativeTransform` (`self.DefaultSceneRoot`)) (`|GetArrayItem` (`self.CameraLock`) (`local.NextIndex`))))
      (`KismetSystemLibrary.DrawDebugLine` (`local.World PointA`) (`local.World PointB`) (struct :`R` 0.193407 :`G` 1.0 :`A` 1.0) 0.0 10.0))))

(fn `UserConstructionScript`
  (set `SpringArmComponent.TargetArmLength` (`self.Target Arm Length`) (`self.SpringArm`))
  (`self.DrawDebugLine`))