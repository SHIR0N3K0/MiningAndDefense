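; BP_TimeBoard is a train station departure board whose readouts for next train, service name, time and platform are configurable.
; The construction script copies each text variable into a front and reverse text component, so both sides show the same information.
; It also applies a configurable scrolling material to a material slot on the board mesh.
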(fn `UserConstructionScript`
  ;[1 1 1] This is the readout to set all the board's information
  ;;[1 1 1] These components set the board's different text variables.
  (`TextRenderComponent.K2_SetText` (`self.Next Train Font`) (`self.Next Train Text`))
  (`TextRenderComponent.K2_SetText` (`self.Next Train Font Reverse`) (`self.Next Train Text`))
  (`TextRenderComponent.K2_SetText` (`self.Train Service Name`) (`self.Train Service Text`))
  (`TextRenderComponent.K2_SetText` (`self.Train Service Reverse`) (`self.Train Service Text`))
  (`TextRenderComponent.K2_SetText` (`self.Time`) (`self.Time Text`))
  (`TextRenderComponent.K2_SetText` (`self.Time Reverse`) (`self.Time Text`))
  (`TextRenderComponent.K2_SetText` (`self.Platform`) (`self.Platform Number`))
  (`TextRenderComponent.K2_SetText` (`self.Platform Reverse`) (`self.Platform Number`))
  ;;[1 1 1] This component sets the board's scrolling material
  (`PrimitiveComponent.SetMaterial` (`self.SM_TimeBoard_01a`) 1 (`self.Scrolling Texture Mat`)))