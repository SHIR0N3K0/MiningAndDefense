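; BP_TrafficLight is a decorative train station signal that cycles endlessly through red, red with blue, green and blue lights.
; The construction script hides the green and blue cone meshes, leaving red as the starting light.
; BeginPlay runs a chain of fixed Delays and visibility toggles that wires back to its start, with no Tick or external input driving it.
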(event `self.ReceiveBeginPlay`
  (bind _sm_trafficlights_green (`self.SM_TrafficLights_Green`))
  (bind _sm_trafficlights_blue (`self.SM_TrafficLights_Blue`))
  ;[1 1 1] This script is fairly straightforward, it simply runs through and changes the visibility of three traffic light cones, and then once it's finished it resets to the beginning. Not ideal for actual working lights, but gives a nice effect.
  (`KismetSystemLibrary.Delay` 2.0 :!label _label)
  (`SceneComponent.SetVisibility` (`self.SM_TrafficLights_Blue`) true false)
  (`KismetSystemLibrary.Delay` 3.0)
  (`SceneComponent.SetVisibility` (`self.SM_TrafficLights_Green`) true false)
  (`SceneComponent.SetVisibility` _sm_trafficlights_blue false false)
  (`SceneComponent.SetVisibility` (`self.SM_TrafficLights_Red`) false false)
  (`SceneComponent.SetVisibility` _sm_trafficlights_green true false)
  (`KismetSystemLibrary.Delay` 5.0)
  (`SceneComponent.SetVisibility` _sm_trafficlights_green false false)
  (`SceneComponent.SetVisibility` _sm_trafficlights_blue true false)
  (`KismetSystemLibrary.Delay` 3.0)
  (`SceneComponent.SetVisibility` _sm_trafficlights_blue false false)
  (`SceneComponent.SetVisibility` (`self.SM_TrafficLights_Red`) true false)
  (goto _label))

(fn `UserConstructionScript`
  (`SceneComponent.SetVisibility` (`self.SM_TrafficLights_Green`) false false)
  (`SceneComponent.SetVisibility` (`self.SM_TrafficLights_Blue`) false false))