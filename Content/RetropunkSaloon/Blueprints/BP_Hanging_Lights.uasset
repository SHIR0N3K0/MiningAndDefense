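; BP_Hanging_Lights is a placeable actor that lays strings of hanging lights along an editable spline.
; Its construction script divides the spline by SectionLength and adds a spline mesh component for each section, each using a random variant from the Meshes array.
; Each piece follows the spline's positions and tangents in local space, with tangents clamped to the section length.
; The event graph holds no active logic.
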(fn `UserConstructionScript`
  (locals (`Spline Mesh Comp` :type "SplineMeshComponent Object Reference"))
  (bind _spline (`self.Spline`))
  (bind _meshes (`self.Meshes`))
  (for _index (range (+ (`KismetMathLibrary.FTrunc` (/ (`SplineComponent.GetSplineLength` (`self.Spline`)) (`self.SectionLength`))) 1))
    (bind _returnvalue (`AddComponent|NODE_AddSplineMeshComponent-0`))
    (`StaticMeshComponent.SetStaticMesh` _returnvalue (`|GetArrayItem` _meshes (`KismetMathLibrary.RandomInteger` (`KismetArrayLibrary.Array_Length` _meshes))))
    (`SplineMeshComponent.SetForwardAxis` _returnvalue "X" true)
    (bind _returnvalue_2 (* _index (`self.SectionLength`)))
    (bind _returnvalue_3 (* (+ _index 1) (`self.SectionLength`)))
    (`SplineMeshComponent.SetStartAndEnd` _returnvalue (`SplineComponent.GetLocationAtDistanceAlongSpline` _spline _returnvalue_2 "Local") (`KismetMathLibrary.ClampVectorSize` (`SplineComponent.GetTangentAtDistanceAlongSpline` _spline _returnvalue_2 "Local") 0.0 (`self.SectionLength`)) (`SplineComponent.GetLocationAtDistanceAlongSpline` _spline _returnvalue_3 "Local") (`KismetMathLibrary.ClampVectorSize` (`SplineComponent.GetTangentAtDistanceAlongSpline` _spline _returnvalue_3 "Local") 0.0 (`self.SectionLength`)) true)))